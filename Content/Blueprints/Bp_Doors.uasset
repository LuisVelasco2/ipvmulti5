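; Networked door actor that is randomly real or fake, opening when a player character touches a real one.
; On BeginPlay the server flips a random bool into RealDoor and forces a net update.
; When a BP_ThirdPersonCharacter overlaps the Box, the server checks RealDoor and, if true, hides Cube1 and disables its collision.
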(event `self.ReceiveBeginPlay`
  (if (`KismetSystemLibrary.IsServer`)
    (`self.UpdateRandomDoors`)))

(event `UpdateRandomDoors`
  (if (`KismetMathLibrary.RandomBool`)
    (set `self.RealDoor` true)
    (else
      (set `self.RealDoor` false)))
  (`self.ForceNetUpdate`))

(event `self.Box.OnComponentBeginOverlap`
  (params (OverlappedComponent :type "PrimitiveComponent Object Reference") (OtherActor :type "Actor Object Reference") (OtherComp :type "PrimitiveComponent Object Reference") (OtherBodyIndex :type Integer) (bFromSweep :type Boolean) (SweepResult :type "HitResult Structure (by ref)"))
  (cast `/Game/ThirdPerson/Blueprints/BP_ThirdPersonCharacter` OtherActor)
  (if (`KismetSystemLibrary.IsServer`)
    (if (`self.RealDoor`)
      (`self.UpdateDoorVIsibility`))))

(event `UpdateDoorVIsibility`
  (`SceneComponent.SetHiddenInGame` (`self.Cube1`) true false)
  (`PrimitiveComponent.SetCollisionEnabled` (`self.Cube1`) "NoCollision"))

(fn `UserConstructionScript`)