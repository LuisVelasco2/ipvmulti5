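; Spawner actor that periodically creates launch pads at its own transform.
; BeginPlay starts a looping two-second timer, and the spawn event runs only on the server.
; Each spawned BP_LaunchPad is told to move and given a configurable lifespan, so it destroys itself later.
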(event `self.ReceiveBeginPlay`
  (`KismetSystemLibrary.K2_SetTimerDelegate` (`|CreateDelegate` :!event `SpawnLauncPad`) 2.0 true))

(event `SpawnLauncPad`
  (if (`KismetSystemLibrary.IsServer`)
    (bind _returnvalue (`|SpawnActorFromClass` "/Game/Blueprints/Actors/BP_LaunchPad.BP_LaunchPad_C" (`self.GetTransform`) "Undefined" "MultiplyWithRoot" null null))
    (bind _output_get (set `self.LaunchPad` _returnvalue))
    (`/Game/Blueprints/Actors/BP_LaunchPad.MoveLaunchpad` _output_get)
    (`self.SetLifeSpan` (`self.LaunchPad`) (`self.LifespanLaunchPad`))))

(fn `UserConstructionScript`)