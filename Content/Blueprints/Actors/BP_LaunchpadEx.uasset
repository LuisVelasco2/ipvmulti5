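; Launchpad actor that throws the third-person character when it overlaps the pad's Box.
; The launch direction is the actor's rotation with a pitch offset, scaled by a force, and it overrides the character's existing velocity on all axes.
; An optional spin adds a local rotation to the Box every tick, using the actor's roll and pitch and a set yaw step as deltas, without delta-time scaling.
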(event `self.ReceiveTick`
  (params (DeltaSeconds :type "Float (single-precision)"))
  (if (`self.bShouldRotate`)
    (`self.UpdateActorRotation`)))

(event `self.Box.OnComponentBeginOverlap`
  (params (OverlappedComponent :type "PrimitiveComponent Object Reference") (OtherActor :type "Actor Object Reference") (OtherComp :type "PrimitiveComponent Object Reference") (OtherBodyIndex :type Integer) (bFromSweep :type Boolean) (SweepResult :type "HitResult Structure (by ref)"))
  (bind _asbp_third_person_character (cast `/Game/ThirdPerson/Blueprints/BP_ThirdPersonCharacter` OtherActor))
  (`Character.LaunchCharacter` _asbp_third_person_character (`self.GetLaunchDirection`) true true))

(fn `GetLaunchDirection`
  (returns (launchDirection :type "Vector Structure"))
  (bind (_launchdirection_roll _launchdirection_pitch _launchdirection_yaw) (`KismetMathLibrary.BreakRotator` (`self.LaunchDirection`)))
  (set `self.LaunchDirection` (`self.K2_GetActorRotation`))
  (set `self.LaunchDirection` (`KismetMathLibrary.MakeRotator` _launchdirection_roll (+ _launchdirection_pitch (`self.LaunchAngle`)) _launchdirection_yaw))
  (bind _output_get (set `self.LaunchVelocity` (* (`KismetMathLibrary.GetForwardVector` (`self.LaunchDirection`)) (`self.LaunchForce`))))
  (return _output_get))

(fn `UpdateActorRotation`
  (bind (_returnvalue_roll _returnvalue_pitch) (`KismetMathLibrary.BreakRotator` (`self.K2_GetActorRotation`)))
  (`SceneComponent.K2_AddLocalRotation` (`self.Box`) (`KismetMathLibrary.MakeRotator` _returnvalue_roll _returnvalue_pitch (`self.NewRotationZ`)) false false))

(fn `UserConstructionScript`)