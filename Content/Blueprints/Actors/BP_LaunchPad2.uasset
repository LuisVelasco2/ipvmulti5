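; BP_LaunchPad2 is a launch pad actor that throws the third-person character when it steps into the pad's box trigger.
; On overlap it calls LaunchCharacter along the pad's forward direction, pitched by LaunchAngle and scaled by LaunchForce, adding to existing velocity rather than overriding it.
; An optional Rotation flag spins the pad in yaw every tick, so the launch direction turns with it.
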(event `self.ReceiveTick`
  (params (DeltaSeconds :type "Float (single-precision)"))
  (if (`self.Rotation`)
    (`self.K2_AddActorLocalRotation` (`KismetMathLibrary.MakeRotator` 0.0 0.0 1.0))))

(event `self.Box.OnComponentBeginOverlap`
  (params (OverlappedComponent :type "PrimitiveComponent Object Reference") (OtherActor :type "Actor Object Reference") (OtherComp :type "PrimitiveComponent Object Reference") (OtherBodyIndex :type Integer) (bFromSweep :type Boolean) (SweepResult :type "HitResult Structure (by ref)"))
  (bind _asbp_third_person_character (cast `/Game/ThirdPerson/Blueprints/BP_ThirdPersonCharacter` OtherActor))
  (`KismetSystemLibrary.PrintString` "lanzado")
  (`Character.LaunchCharacter` _asbp_third_person_character (* (`KismetMathLibrary.GetForwardVector` (`KismetMathLibrary.MakeRotator` (.roll (`self.K2_GetActorRotation`)) (+ (.pitch (`self.K2_GetActorRotation`)) (`self.LaunchAngle`)) (.yaw (`self.K2_GetActorRotation`)))) (`self.LaunchForce`)) false false))

(fn `UserConstructionScript`)