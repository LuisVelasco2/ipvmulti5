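; BP_LaunchPad is a launch pad actor that moves along its forward vector when its MoveLaunchpad event is triggered.
; The event slows a timeline's play rate, then uses its Alfa track to lerp toward a point ahead with a swept move.
; Both lerp endpoints are re-read from the current location each update, so movement accumulates instead of spanning a fixed distance.
; The file contains no player-launching logic.
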(event `self.ReceiveBeginPlay`)

(event `MoveLaunchpad`
  (`TimelineComponent.SetPlayRate` (`self.Timeline_MoveLaunchpad`) (/ 1.0 200.0))
  (bind (_direction _alfa) (`Timeline|Timeline_MoveLaunchpad`)
    (:`Update`
      (`self.K2_SetActorLocation` (`KismetMathLibrary.VLerp` (`self.K2_GetActorLocation`) (+ (`self.K2_GetActorLocation`) (* (`KismetMathLibrary.GetForwardVector` (`self.K2_GetActorRotation`)) 400.0)) _alfa) true))))

(fn `UserConstructionScript`)